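; Base FPS character Blueprint that handles player UI, damage forwarding and debug session controls.
; BeginPlay adds the GamePlay widget without a local-control check, and any damage passes to TakeDamageCustom.
; Tick polls RepIsDead on the locally controlled pawn to open WBP_PauseMenu once with UI-only input, as the Pause action also does on release.
; Numpad keys call FPSGameInstance to create, find or destroy-and-quit sessions, and fetch friends.
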(event EventBeginPlay
  (bind _returnvalue (UserInterface|CreateWidget "/Game/UI/GamePlay.GamePlay_C"))
  (UserInterface|Viewport|AddtoViewport _returnvalue 0))

(event Collision|EventActorBeginOverlap
  (params (OtherActor :type Actor%20Object%20Reference)))

(event EventTick
  (params (DeltaSeconds :type Float%20%28single-precision%29))
  (bind _returnvalue (Game|GetPlayerController 0))
  (if (Pawn|IsLocallyControlled)
    (if (Variables|Default|GetRep_IsDead)
      (if (not (Variables|Default|GetUI%20Created))
        (bind _returnvalue_2 (UserInterface|CreateWidget "/Game/UI/WBP_PauseMenu.WBP_PauseMenu_C" (Game|GetPlayerController 0)))
        (UserInterface|Viewport|AddtoViewport _returnvalue_2 0)
        (Input|SetInputModeUIOnly _returnvalue _returnvalue_2 "DoNotLock")
        (Variables|/Script/Engine.PlayerController|SetbShowMouseCursor _returnvalue true)
        (Variables|Default|SetUI%20Created true)))))

(event Game|Damage|EventAnyDamage
  (params (Damage :type Float%20%28single-precision%29) (DamageType :type Damage%20Type%20Object%20Reference) (InstigatedBy :type Controller%20Object%20Reference) (DamageCauser :type Actor%20Object%20Reference))
  (Class|FPSBaseCharacter|TakeDamageCustom Damage))

(event Input|ActionEvents|InputActionPause
  (params (Key :type Key%20Structure :default "None"))
  (bind _returnvalue (Game|GetPlayerController 0))
  (:Released
    (bind _returnvalue_2 (UserInterface|CreateWidget "/Game/UI/WBP_PauseMenu.WBP_PauseMenu_C"))
    (UserInterface|Viewport|AddtoViewport _returnvalue_2 0)
    (Input|SetInputModeUIOnly _returnvalue _returnvalue_2 "DoNotLock")
    (Variables|/Script/Engine.PlayerController|SetbShowMouseCursor _returnvalue true)))

(event Input|KeyboardEvents|NumPadOne
  (params (Key :type Key%20Structure :default "None"))
  (:Pressed
    (bind _asfpsgame_instance (Utilities|Casting|CastToFPSGameInstance (Game|GetGameInstance)))
    (Class|FPSGameInstance|CreateSession _asfpsgame_instance)))

(event Input|KeyboardEvents|NumPadTwo
  (params (Key :type Key%20Structure :default "None"))
  (:Pressed
    (bind _asfpsgame_instance (Utilities|Casting|CastToFPSGameInstance (Game|GetGameInstance)))
    (Class|FPSGameInstance|DestroySession _asfpsgame_instance)
    (Utilities|FlowControl|Delay 0.5)
    (Game|QuitGame 0 "Quit" false)))

(event Input|KeyboardEvents|NumPadThree
  (params (Key :type Key%20Structure :default "None"))
  (:Pressed
    (bind _asfpsgame_instance (Utilities|Casting|CastToFPSGameInstance (Game|GetGameInstance)))
    (Class|FPSGameInstance|GetAllFriends _asfpsgame_instance)))

(event Input|KeyboardEvents|NumPadFour
  (params (Key :type Key%20Structure :default "None"))
  (:Pressed
    (bind _asfpsgame_instance (Utilities|Casting|CastToFPSGameInstance (Game|GetGameInstance)))
    (Class|FPSGameInstance|FindSession _asfpsgame_instance)))

(fn ConstructionScript)